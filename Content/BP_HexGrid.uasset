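; BP_HexGrid is a hex grid actor, apparently an unfinished manager for tile data.
; BeginPlay runs empty nested loops over grid width and height, then finds and casts the BP_HexGridVisual actor without using it.
; A disconnected chain would fill GridData with each tile's coordinates and world position from HexGridComponent's GridToWorld, but it never runs.
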(event `self.ReceiveBeginPlay`
  (for _index (range (`self.GridWidth`))
    (for _index_2 (range (`self.GridHeight`))
      _))
  (bind _returnvalue (`GameplayStatics.GetActorOfClass` "/Game/BlueprintClasses/BP_HexGridVisual.BP_HexGridVisual_C"))
  (cast `/Game/BlueprintClasses/BP_HexGridVisual` _returnvalue))

(fn `UserConstructionScript`)