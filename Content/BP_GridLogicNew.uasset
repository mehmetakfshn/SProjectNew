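; Hex grid actor that builds a terrain map from instanced static meshes in its construction script.
; Nested X/Y loops place pointy-top hexes, shifting odd rows by half a tile.
; A bitwise test on index remainders picks mountains and the rest become grass, as the water test for index zero never matches loops starting at one.
; GridData tile-record writes are disconnected, and the event graph is empty.
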(fn `UserConstructionScript`
  ; x
  (for _index (range 1 (+ (`self.Number on X`) 1))
    ; Y
    (for _index_2 (range 1 (+ (`self.Number on Y`) 1))
      (if (== (`KismetMathLibrary.And_IntInt` (mod _index 5) (mod _index_2 3)) 1)
        (bind _returnvalue (* _index_2 (* (* 100.0 2.0) 0.75)))
        (bind _returnvalue_2 (`KismetMathLibrary.MakeTransform` (`KismetMathLibrary.SelectVector` (`KismetMathLibrary.MakeVector` (* (* 100.0 (`KismetMathLibrary.Sqrt` 3.0)) _index) _returnvalue) (`KismetMathLibrary.MakeVector` (+ (* (* 100.0 (`KismetMathLibrary.Sqrt` 3.0)) _index) (/ (* 100.0 (`KismetMathLibrary.Sqrt` 3.0)) 2.0)) _returnvalue) (== (mod _index_2 2) 0))))
        (`InstancedStaticMeshComponent.AddInstance` (`self.ISM_Mountain`) _returnvalue_2 false)
        (elif (`KismetMathLibrary.Conv_IntToBool` (`KismetMathLibrary.Or_IntInt` (`KismetMathLibrary.Conv_BoolToInt` (== _index 0)) (`KismetMathLibrary.Conv_BoolToInt` (== _index_2 0))))
          (`InstancedStaticMeshComponent.AddInstance` (`self.ISM_Water`) _returnvalue_2 false)
          (elif true
            (`InstancedStaticMeshComponent.AddInstance` (`self.ISM_Grass`) _returnvalue_2 false)))))))